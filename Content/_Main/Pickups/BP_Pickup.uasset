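; BP_Pickup is a world pickup actor that registers itself with a survival character entering its sphere collision.
; On the server, begin overlap gets the character through an interface call and sets itself as its pickup, unless one is already held, which only prints a debug string.
; Separate events disable collision or destroy the actor, and PickupRef returns self.
; End overlap only checks authority and does nothing further.
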(event OnComponentBeginOverlap(SphereCollision)
  (params (OverlappedComponent :type Primitive%20Component%20Object%20Reference) (OtherActor :type Actor%20Object%20Reference) (OtherComp :type Primitive%20Component%20Object%20Reference) (OtherBodyIndex :type Integer) (bFromSweep :type Boolean) (SweepResult :type Hit%20Result%20Structure%20%28by%20ref%29))
  (Networking|SwitchHasAuthority
    (:Authority
      (bind _survivalchar (Class|INTSurvivalCharacter|SurvivalCharRef(Message) OtherActor))
      (Variables|/Game/_Main/BP_SurvivalPlayer.BP_SurvivalPlayer_C|GetPickup _survivalchar
        (:then
          (Development|PrintString "Hello"))
        (:else
          (Default|SRVSetPickup _survivalchar self))))))

(event OnComponentEndOverlap(SphereCollision)
  (params (OverlappedComponent :type Primitive%20Component%20Object%20Reference) (OtherActor :type Actor%20Object%20Reference) (OtherComp :type Primitive%20Component%20Object%20Reference) (OtherBodyIndex :type Integer))
  (Networking|SwitchHasAuthority))

(event Custom|SRV_RemovePickupFromWorld
  (Actor|DestroyActor))

(event Custom|SRV_DisableCollision
  (Collision|SetCollisionEnabled (Variables|Default|GetSphereCollision) "NoCollision"))

(fn ConstructionScript)

(fn PickupRef
  (return self))