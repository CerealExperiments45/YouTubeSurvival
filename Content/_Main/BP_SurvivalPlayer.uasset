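; Networked survival player character Blueprint that handles picking up, firing and aiming a rifle.
; Interact calls a server event that spawns the rifle on the hand socket, removes the pickup, and multicasts a combat-state change to animation and controller-facing rotation.
; Fire forwards to the equipped weapon.
; Aiming drives an FOV zoom timeline and changes walk speed on the server, echoed to the client.
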(event Custom|SRV_AttachWeapon
  (bind _self self)
  ;[1 1 1] AttachWeapon
  (bind _returnvalue (Game|SpawnActorfromClass "/Game/_Main/Pickups/Weapons/Weapon_Rifle.Weapon_Rifle_C" (Transformation|GetActorTransform) "AlwaysSpawn" _self (Variables|Default|GetCamera) _self))
  (bind _output_get (Variables|Default|SetEquippedWeapon _returnvalue))
  (Transformation|AttachComponentToComponent _output_get (Variables|Character|GetMesh) "weapon_r" "SnapToTarget" "SnapToTarget" "SnapToTarget" true)
  (Variables|Default|SetWeaponEquipped true)
  (Default|SRVDisableCollision (Variables|Default|GetPickup))
  (CallFunction|MultiUpdateCombatState 1)
  (Default|SRVRemovePickupfromWorld (Variables|Default|GetPickup)))

(event Custom|Multi_UpdateCombatState
  (params (BlendSpaceInt :type Integer))
  (bind _charactermovement (Variables|Character|GetCharacterMovement))
  ;[1 1 1] UpdateCombatState-Multicast
  (Utilities|FlowControl|Delay 0.2)
  (Class|INTAnimBPPlayer|CombatState(Message) (Components|SkeletalMesh|GetAnimInstance (Variables|Character|GetMesh)) BlendSpaceInt)
  (Variables|/Script/Engine.CharacterMovementComponent|SetbUseControllerDesiredRotation _charactermovement true)
  (Variables|/Script/Engine.CharacterMovementComponent|SetbOrientRotationToMovement _charactermovement false))

(event Custom|SRV_SetPickup
  (params (Pickup :type BP%20Pickup%20Object%20Reference))
  ;[1 1 1] SetPickup
  (Variables|Default|SetPickup Pickup))

(event Custom|SRV_UpdateSpeed
  (params (Speed :type Float%20%28single-precision%29))
  ;[0 0.04577 1] InputAim
  ;;[1 0.1283 0] SRV_Update
  (bind _output_get (Variables|/Script/Engine.CharacterMovementComponent|SetMaxWalkSpeed (Variables|Character|GetCharacterMovement) Speed))
  (CallFunction|ClientUpdateSpeed _output_get))

(event Custom|Client_UpdateSpeed
  (params (Speed :type Float%20%28single-precision%29))
  ;[0 0.04577 1] InputAim
  ;;[1 0.1283 0] SRV_Update
  (Variables|/Script/Engine.CharacterMovementComponent|SetMaxWalkSpeed (Variables|Character|GetCharacterMovement) Speed))

(event EventBeginPlay
  ;[0.4713 0 1] Access Animation
  (|CallParentFunction))

(event Game|Damage|EventPointDamage
  (params (Damage :type Float%20%28single-precision%29) (DamageType :type Damage%20Type%20Object%20Reference) (HitLocation :type Vector :default "0, 0, 0") (HitNormal :type Vector :default "0, 0, 0") (HitComponent :type Primitive%20Component%20Object%20Reference) (BoneName :type Name :default "None") (ShotFromDirection :type Vector :default "0, 0, 0") (InstigatedBy :type Controller%20Object%20Reference) (DamageCauser :type Actor%20Object%20Reference) (HitInfo :type Hit%20Result%20Structure%20%28by%20ref%29))
  ;[1 1 1] PointDamage
)

(event Input|ActionEvents|InputActionInteract
  (params (Key :type Key%20Structure :default "None"))
  ;[1 1 1] Interact Button
  (:Pressed
    (Variables|Default|GetPickup
      (:then
        (CallFunction|SRVAttachWeapon))
      (:else))))

(event Input|ActionEvents|InputActionFireWeapon
  (params (Key :type Key%20Structure :default "None"))
  ;[1 0.3711 0] Input Fire
  (:Pressed
    (bind _equippedweapon (Variables|Default|GetEquippedWeapon)
      (:then
        (Default|SRVFireWeapon _equippedweapon))
      (:else))))

(event Input|ActionEvents|InputActionAim
  (params (Key :type Key%20Structure :default "None"))
  (bind _weaponequipped (Variables|Default|GetWeaponEquipped))
  ;[0 0.04577 1] InputAim
  (:Pressed
    (if _weaponequipped
      (CallFunction|SRVUpdateSpeed 2e+02)
      (bind _time (Timeline|T_FieldOfView PlayFromStart)
        (:Update
          (Camera|SetFieldOfView (Variables|Default|GetCamera) (Math|Interpolation|FInterpTo 9e+01 (Variables|Default|GetFieldOfView) _time (Math|Float|Clamp(Float) (Variables|Default|GetZoomSpeed) 0.1 1e+01)))))))
  (:Released
    (if _weaponequipped
      (CallFunction|SRVUpdateSpeed 5e+02)
      (Timeline|T_FieldOfView Reverse))))

(fn ConstructionScript
  (|CallParentFunction))

(fn SurvivalCharRef
  (return self))