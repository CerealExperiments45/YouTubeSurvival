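; BP_SurvivalController is a player controller that handles walking and looking input and shows the crosshair on screen.
; BeginPlay creates the crosshair widget and adds it to the viewport.
; Move axes apply movement input to the controlled pawn using yaw-only control rotation, while Turn and LookUp feed controller yaw and pitch.
; The SurvivalControllerRef function returns the controller itself.
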(event EventBeginPlay
  (bind _returnvalue (UserInterface|CreateWidget "/Game/_Main/Pickups/Weapons/CrosshairWidge.CrosshairWidge_C"))
  (UserInterface|Viewport|AddtoViewport _returnvalue 0))

(event Input|AxisEvents|InputAxisMoveRight
  (params (AxisValue :type Float%20%28single-precision%29))
  (bind _returnvalue (Pawn|GetControlledPawn))
  ;[0 0.09637 1] InputWalk
  (Utilities|IsValid _returnvalue
    (:Is%20Valid
      (Pawn|Input|AddMovementInput _returnvalue (Math|Vector|GetRightVector (Math|Rotator|MakeRotator 0.0 0.0 (.Yaw (Math|Rotator|BreakRotator (Pawn|GetControlRotation :!class /Script/Engine.Controller))))) AxisValue false))))

(event Input|AxisEvents|InputAxisMoveForward
  (params (AxisValue :type Float%20%28single-precision%29))
  (bind _returnvalue (Pawn|GetControlledPawn))
  ;[0 0.09637 1] InputWalk
  (Utilities|IsValid _returnvalue
    (:Is%20Valid
      (Pawn|Input|AddMovementInput _returnvalue (Math|Vector|GetForwardVector (Math|Rotator|MakeRotator 0.0 0.0 (.Yaw (Math|Rotator|BreakRotator (Pawn|GetControlRotation :!class /Script/Engine.Controller))))) AxisValue false))))

(event Input|AxisEvents|InputAxisTurn
  (params (AxisValue :type Float%20%28single-precision%29))
  ;[0.5024 0 1] InputLook
  (Class|PlayerController|AddYawInput AxisValue))

(event Input|AxisEvents|InputAxisLookUp
  (params (AxisValue :type Float%20%28single-precision%29))
  ;[0.5024 0 1] InputLook
  (Class|PlayerController|AddPitchInput AxisValue))

(fn ConstructionScript)

(fn SurvivalControllerRef
  (return self))